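; BP_InitialBox is a trigger volume actor that tracks whether the player is inside it.
; On overlap begin and end, its Box component sets or clears the BP_Player's IsInTheBox flag and its reference to this box.
; BeginPlay caches the BP_CustomGameInstance, though nothing else in this Blueprint uses it.
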(event OnComponentBeginOverlap(Box)
  (params (OverlappedComponent :type Primitive%20Component%20Object%20Reference) (OtherActor :type Actor%20Object%20Reference) (OtherComp :type Primitive%20Component%20Object%20Reference) (OtherBodyIndex :type Integer) (bFromSweep :type Boolean) (SweepResult :type Hit%20Result%20Structure%20%28by%20ref%29))
  (bind _asbp_player (Utilities|Casting|CastToBP_Player OtherActor))
  (Variables|/Game/Blueprint/Player/BP_Player.BP_Player_C|SetIsInTheBox _asbp_player true)
  (Variables|/Game/Blueprint/Player/BP_Player.BP_Player_C|SetBP_InitialBoxRef _asbp_player self))

(event OnComponentEndOverlap(Box)
  (params (OverlappedComponent :type Primitive%20Component%20Object%20Reference) (OtherActor :type Actor%20Object%20Reference) (OtherComp :type Primitive%20Component%20Object%20Reference) (OtherBodyIndex :type Integer))
  (bind _asbp_player (Utilities|Casting|CastToBP_Player OtherActor))
  (Variables|/Game/Blueprint/Player/BP_Player.BP_Player_C|SetIsInTheBox _asbp_player false)
  (Variables|/Game/Blueprint/Player/BP_Player.BP_Player_C|SetBP_InitialBoxRef _asbp_player 0))

(event EventBeginPlay
  (bind _asbp_custom_game_instance (Utilities|Casting|CastToBP_CustomGameInstance (Game|GetGameInstance)))
  (Variables|Default|SetAs%20BP%20Custom%20Game%20Instance _asbp_custom_game_instance))

(event Collision|EventActorBeginOverlap
  (params (OtherActor :type Actor%20Object%20Reference)))

(event EventTick
  (params (DeltaSeconds :type Float%20%28single-precision%29)))

(fn ConstructionScript)