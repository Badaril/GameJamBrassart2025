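; BP_Gougoutte is an actor that falls straight down in an endless loop, apparently a looping droplet.
; BeginPlay stores the starting location and calls Down, which plays a Timeline that lowers the actor a fixed step on each update.
; When the Timeline finishes, the actor snaps back to its start and Down calls itself again.
; The step ignores delta time, so fall speed and distance depend on frame rate.
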(event Custom|Down
  (Timeline|Timeline PlayFromStart
    (:Update
      (Transformation|SetActorLocation (- (Transformation|GetActorLocation) "0.000000,0.000000,10.000000") false false))
    (:Finished
      (Transformation|SetActorLocation (Variables|Default|GetStartingLocation) false false)
      (CallFunction|Down))))

(event EventBeginPlay
  (|CallParentFunction)
  (Variables|Default|SetStartingLocation (Transformation|GetActorLocation))
  (CallFunction|Down))

(event Collision|EventActorBeginOverlap
  (params (OtherActor :type Actor%20Object%20Reference))
  (|CallParentFunction OtherActor) ; This node is disabled and will not be called.\nDrag off pins to build functionality.
)

(event EventTick
  (params (DeltaSeconds :type Float%20%28single-precision%29))
  (|CallParentFunction DeltaSeconds) ; This node is disabled and will not be called.\nDrag off pins to build functionality.
)

(fn ConstructionScript
  (|CallParentFunction))