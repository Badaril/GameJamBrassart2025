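; BP_TimedDamageBox is an actor that cycles a Box component on and off on a repeating timer, as a timed hazard volume by its name.
; BeginPlay starts the custom Trigger event, which waits, enables collision and shows the box briefly, then disables and hides it.
; Trigger calls itself after a final delay to loop indefinitely.
; The graph itself applies no damage.
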(event Custom|Trigger
  (bind _box (Variables|Default|GetBox))
  (bind _box_2 (Variables|Default|GetBox))
  (Utilities|FlowControl|Delay 0.8)
  (Collision|SetCollisionEnabled _box_2 "QueryAndPhysics")
  (Development|SetHiddeninGame _box_2 false false)
  (Utilities|FlowControl|Delay 0.2)
  (Collision|SetCollisionEnabled _box "NoCollision")
  (Development|SetHiddeninGame _box true false)
  (Utilities|FlowControl|Delay 1.2)
  (CallFunction|Trigger))

(event EventBeginPlay
  (|CallParentFunction)
  (CallFunction|Trigger))

(event Collision|EventActorBeginOverlap
  (params (OtherActor :type Actor%20Object%20Reference))
  (|CallParentFunction OtherActor) ; This node is disabled and will not be called.\nDrag off pins to build functionality.
)

(event EventTick
  (params (DeltaSeconds :type Float%20%28single-precision%29))
  (|CallParentFunction DeltaSeconds))

(fn ConstructionScript
  (|CallParentFunction))