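; BP_TargetBox is the destination actor where a mushroom helper (BP_BBChampignon) resolves the action of its linked InitialBox.
; When the game instance's OnBoxOverlap fires, it spawns the mushroom at InitialBox, destroys that box and passes itself as target.
; After a fixed delay, it removes the mushroom, then spawns a bounce pad or platform, or shrinks WoodObstacleRef in steps and disables collision.
; AnimationChampi lerps BBChampiRef toward the target but is not called here.
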(event Custom|Change
  (bind _woodobstacleref (Variables|Default|GetWoodObstacleRef))
  (bind _cube (Variables|/Game/Ilian/BP_WoodObstacle.BP_WoodObstacle_C|GetCube _woodobstacleref))
  (switch Utilities|FlowControl|Switch|SwitchonE_TypeOfActionBBChampi (Variables|/Game/Blueprint/BP_InitialBox.BP_InitialBox_C|GetTypeOfAction (Variables|Default|GetInitialBox))
    (:NewEnumerator0
      ;[1 1 1] Spawn le BB champi et se déplace vers la target box pour spawn un trampoline
      (Development|PrintString "TRAMPOLINE")
      (bind _returnvalue (Game|SpawnActorfromClass "/Game/Ilian/BP_BBChampignon.BP_BBChampignon_C" (Math|Transform|MakeTransform (Transformation|GetActorLocation (Variables|Default|GetInitialBox)) "0, 0, 0" "1.000000,1.000000,1.000000") "Undefined" "MultiplyWithRoot" 0 0))
      (Actor|DestroyActor (Variables|Default|GetInitialBox))
      (Variables|/Game/Ilian/BP_BBChampignon.BP_BBChampignon_C|SetTargetBoxRef _returnvalue self)
      (Utilities|FlowControl|Delay 0.5) ; A changer en fonction de la distance entre l'initial box et la target box
      (Actor|DestroyActor _returnvalue)
      (Game|SpawnActorfromClass "/Game/Ilian/BP_BouncePad.BP_BouncePad_C" (Math|Transform|MakeTransform (Transformation|GetActorLocation) "0, 0, 0" "1.000000,1.000000,1.000000") "Undefined" "MultiplyWithRoot" 0 0))
    (:NewEnumerator1
      ;[1 1 1] Spawn le BB champi et se déplace vers la target box pour détruire le morceau de bois
      (Development|PrintString "MIAM MIAM MIAM")
      (bind _returnvalue_2 (Game|SpawnActorfromClass "/Game/Ilian/BP_BBChampignon.BP_BBChampignon_C" (Math|Transform|MakeTransform (Transformation|GetActorLocation (Variables|Default|GetInitialBox)) "0, 0, 0" "1.000000,1.000000,1.000000") "Undefined" "MultiplyWithRoot" 0 0))
      (Actor|DestroyActor (Variables|Default|GetInitialBox))
      (Variables|/Game/Ilian/BP_BBChampignon.BP_BBChampignon_C|SetTargetBoxRef _returnvalue_2 self)
      (Utilities|FlowControl|Delay 0.5) ; A changer en fonction de la distance entre l'initial box et la target box
      (Actor|DestroyActor _returnvalue_2)
      (Transformation|SetRelativeScale3D _cube (Math|Vector|MakeVector 1.0 1.0 1.0))
      (Utilities|FlowControl|Delay 0.5)
      (Transformation|SetRelativeScale3D (Variables|/Game/Ilian/BP_WoodObstacle.BP_WoodObstacle_C|GetCube (Variables|Default|GetWoodObstacleRef)) (Math|Vector|MakeVector 1.0 1.0 0.5))
      (Utilities|FlowControl|Delay 0.5)
      (Transformation|SetRelativeScale3D (Variables|/Game/Ilian/BP_WoodObstacle.BP_WoodObstacle_C|GetCube (Variables|Default|GetWoodObstacleRef)) (Math|Vector|MakeVector 0.0 0.0 0.0))
      (Collision|SetCollisionEnabled _cube "NoCollision"))
    (:NewEnumerator2
      ;[1 1 1] Spawn le BB champi et se déplace vers la target box pour spawn une plateforme
      (Development|PrintString "PLATEFORME")
      (bind _returnvalue_3 (Game|SpawnActorfromClass "/Game/Ilian/BP_BBChampignon.BP_BBChampignon_C" (Math|Transform|MakeTransform (Transformation|GetActorLocation (Variables|Default|GetInitialBox)) "0, 0, 0" "1.000000,1.000000,1.000000") "Undefined" "MultiplyWithRoot" 0 0))
      (Actor|DestroyActor (Variables|Default|GetInitialBox))
      (Variables|/Game/Ilian/BP_BBChampignon.BP_BBChampignon_C|SetTargetBoxRef _returnvalue_3 self)
      (Utilities|FlowControl|Delay 0.5) ; A changer en fonction de la distance entre l'initial box et la target box
      (Actor|DestroyActor _returnvalue_3)
      (Game|SpawnActorfromClass "/Game/Ilian/BP_Plateforme.BP_Plateforme_C" (Math|Transform|MakeTransform (Transformation|GetActorLocation) "0, 0, 0" "1.000000,1.000000,1.000000") "Undefined" "MultiplyWithRoot" 0 0))))

(event EventBeginPlay
  (bind _asbp_custom_game_instance (Utilities|Casting|CastToBP_CustomGameInstance (Game|GetGameInstance)))
  (bind _output_get (Variables|Default|SetAs%20BP%20Custom%20Game%20Instance _asbp_custom_game_instance))
  (EventDispatchers|BindEventtoOnBoxOverlap _output_get (delegate Custom|Change)))

(event Collision|EventActorBeginOverlap
  (params (OtherActor :type Actor%20Object%20Reference)))

(event EventTick
  (params (DeltaSeconds :type Float%20%28single-precision%29)))

(fn ConstructionScript)

(fn AnimationChampi
  (Transformation|SetActorLocation (Variables|Default|GetBBChampiRef) (Math|Vector|Lerp(Vector) (Transformation|GetActorLocation (Variables|Default|GetBBChampiRef)) (Transformation|GetActorLocation) 0.1) true false))