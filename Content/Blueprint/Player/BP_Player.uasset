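; Player character for a 2D side-view game, with walking, jumping and a box-switching power.
; BeginPlay registers the Enhanced Input mapping context, caches the custom game instance and displays the timer widget.
; Movement runs along world X, flipping the sprite through control rotation, while Tick picks idle, walk, rise or fall flipbooks from velocity and ground state.
; The power calls Change on the referenced box's target while IsInTheBox is true.
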(event Input|EnhancedActionEvents|EnhancedInputActionIA_Jump2D
  (params (ActionValue :type Boolean) (ElapsedSeconds :type Float%20%28double-precision%29) (TriggeredSeconds :type Float%20%28double-precision%29) (InputAction :type Input%20Action%20Object%20Reference :default "/Game/Blueprint/Player/Inputs/IA_Jump2D.IA_Jump2D"))
  ;[1 1 1] Saut
  (:Started
    (Character|Jump))
  (:Completed
    (Character|StopJumping)))

(event Input|EnhancedActionEvents|EnhancedInputActionIA_Move2D
  (params (ActionValue :type Float%20%28double-precision%29) (ElapsedSeconds :type Float%20%28double-precision%29) (TriggeredSeconds :type Float%20%28double-precision%29) (InputAction :type Input%20Action%20Object%20Reference :default "/Game/Blueprint/Player/Inputs/IA_Move2D.IA_Move2D"))
  ;[1 1 1] Déplacements
  (Pawn|Input|AddMovementInput "1.000000,0.000000,0.000000" ActionValue false)
  ;;[1 1 1] Retourner le sprite si il va a gauche
  (Pawn|SetControlRotation (Pawn|GetController) (select (> ActionValue 0.0) (Math|Rotator|MakeRotator 0.0 0.0 0.0) (Math|Rotator|MakeRotator 0.0 0.0 1.8e+02))))

(event Input|EnhancedActionEvents|EnhancedInputActionIA_Power
  (params (ActionValue :type Boolean) (ElapsedSeconds :type Float%20%28double-precision%29) (TriggeredSeconds :type Float%20%28double-precision%29) (InputAction :type Input%20Action%20Object%20Reference :default "/Game/Ilian/IA_Power.IA_Power"))
  (:Started
    (if (Variables|Default|GetIsInTheBox)
      (Default|Change (Variables|/Game/Blueprint/BP_InitialBox.BP_InitialBox_C|GetTargetBox (Variables|Default|GetBP_InitialBoxRef))))))

(event EventBeginPlay
  ;[1 1 1] J'attribue à mon Player la fiche d'inputs que j'ai créé (IMC_Player). Ca me permet d'avoir accès aux Inputs Action
  (bind _asplayer_controller (Utilities|Casting|CastToPlayerController (Pawn|GetController)))
  (Input|AddMappingContext (PlayerController|LocalPlayerSubsystems|GetEnhancedInputLocalPlayerSubsystem _asplayer_controller) "/Game/Blueprint/Player/Inputs/IMC_Player.IMC_Player" 0 "(bIgnoreAllPressedKeysUntilRelease=True,bForceImmediately=False,bNotifyUserSettings=False)")
  (bind _asbp_custom_game_instance (Utilities|Casting|CastToBP_CustomGameInstance (Game|GetGameInstance)))
  (Variables|Default|SetAs%20BP%20Custom%20Game%20Instance _asbp_custom_game_instance)
  (bind _returnvalue (UserInterface|CreateWidget "/Game/Blueprint/Interface/WBP_Timer.WBP_Timer_C"))
  (UserInterface|Viewport|AddtoViewport _returnvalue 0))

(event Collision|EventActorBeginOverlap
  (params (OtherActor :type Actor%20Object%20Reference)))

(event EventTick
  (params (DeltaSeconds :type Float%20%28single-precision%29))
  ;[1 1 1] Obligatoire sur le tick car on utilise un flipbook 2D (AnimBlueprint pour 3D)
  (CallFunction|UpdateAnimations))

(fn ConstructionScript)

(fn UpdateAnimations
  (if (AI|Components|NavMovement|IsMovingonGround (Variables|Character|GetCharacterMovement))
    (if (> (Math|Vector|VectorLength (Transformation|GetVelocity)) 0.0)
      (Sprite|SetFlipbook (Variables|Default|GetSprite) "/Game/Blueprint/Player/AnimsDef/Anim_WalkPlayer.Anim_WalkPlayer")
      (else
        (Sprite|SetFlipbook (Variables|Default|GetSprite) "/Game/Blueprint/Player/AnimsDef/Anim_IdlePlayer.Anim_IdlePlayer")))
    (elif (< (.z (Transformation|GetVelocity)) 0.0)
      (Sprite|SetFlipbook (Variables|Default|GetSprite) "/Game/Blueprint/Player/AnimsDef/Anim_JumpFall.Anim_JumpFall")
      (else
        (Sprite|SetFlipbook (Variables|Default|GetSprite) "/Game/Blueprint/Player/AnimsDef/Anim_JumpRise.Anim_JumpRise")))))