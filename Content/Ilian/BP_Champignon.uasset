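; BP_Champignon is a mushroom-themed Blueprint holding a draft of a power that turns a spawned BP_BBChampignon into a bounce pad, currently inactive.
; The IA_Power input event is empty, and the spawn chain is disconnected, so it never runs.
; That chain spawns BP_BBChampignon at the actor's location, waits briefly, records a point below it, destroys it and spawns BP_BouncePad there.
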(event Input|EnhancedActionEvents|EnhancedInputActionIA_Power
  (params (ActionValue :type Boolean) (ElapsedSeconds :type Float%20%28double-precision%29) (TriggeredSeconds :type Float%20%28double-precision%29) (InputAction :type Input%20Action%20Object%20Reference :default "/Game/Ilian/IA_Power.IA_Power")))

(event EventBeginPlay
  (|CallParentFunction) ; This node is disabled and will not be called.\nDrag off pins to build functionality.
)

(event Collision|EventActorBeginOverlap
  (params (OtherActor :type Actor%20Object%20Reference)))

(event EventTick
  (params (DeltaSeconds :type Float%20%28single-precision%29)))

(fn ConstructionScript
  (|CallParentFunction))