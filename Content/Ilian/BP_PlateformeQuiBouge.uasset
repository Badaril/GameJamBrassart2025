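; Moving platform actor that shuttles back and forth along the world X axis.
; On BeginPlay, after short delays, it scales three plane components, offsets two of them in opposite X directions, hides all three, then starts moving.
; Right and Left events each play a Timeline and chain into each other endlessly.
; Each Timeline update adds a fixed offset without reading a track value, so speed depends on frame rate.
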(event Custom|Right
  (Timeline|Timeline PlayFromStart
    (:Update
      (Transformation|SetActorLocation (+ (Transformation|GetActorLocation) "2.000000,0.000000,0.000000") false false))
    (:Finished
      (CallFunction|Left))))

(event Custom|Left
  (Timeline|Timeline_0 PlayFromStart
    (:Update
      (Transformation|SetActorLocation (- (Transformation|GetActorLocation) "2.000000,0.000000,0.000000") false false))
    (:Finished
      (CallFunction|Right))))

(event EventBeginPlay
  (bind _plane1 (Variables|Default|GetPlane1))
  (bind _plane2 (Variables|Default|GetPlane2))
  (Utilities|FlowControl|Delay 0.15)
  (Transformation|SetWorldScale3D (Variables|Default|GetPlane) "2.500000,2.500000,2.500000")
  (Transformation|SetWorldScale3D (Variables|Default|GetPlane1) "2.500000,2.500000,2.500000")
  (Transformation|SetWorldScale3D (Variables|Default|GetPlane2) "2.500000,2.500000,2.500000")
  (Transformation|SetWorldLocation _plane1 (- (Transformation|GetWorldLocation _plane1) "50.000000,0.000000,0.000000") false false)
  (Transformation|SetWorldLocation _plane2 (+ (Transformation|GetWorldLocation _plane2) "50.000000,0.000000,0.000000") false false)
  (Utilities|FlowControl|Delay 0.15)
  (Rendering|SetVisibility (Variables|Default|GetPlane) false false)
  (Rendering|SetVisibility (Variables|Default|GetPlane1) false false)
  (Rendering|SetVisibility (Variables|Default|GetPlane2) false false)
  (CallFunction|Right))

(event Collision|EventActorBeginOverlap
  (params (OtherActor :type Actor%20Object%20Reference)))

(event EventTick
  (params (DeltaSeconds :type Float%20%28single-precision%29)))

(fn ConstructionScript)