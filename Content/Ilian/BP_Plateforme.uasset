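; BP_Plateforme is a platform actor, judging by its name, that briefly enlarges and then hides its visuals when play begins.
; After a short delay, BeginPlay sets a larger world scale on a plane and two static meshes and shifts the meshes in opposite directions along world X.
; A second delay precedes hiding all three components without propagating to children.
; Tick, overlap and construction logic are empty.
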(event EventBeginPlay
  (bind _staticmesh (Variables|Default|GetStaticMesh))
  (bind _staticmesh1 (Variables|Default|GetStaticMesh1))
  (Utilities|FlowControl|Delay 0.15)
  (Transformation|SetWorldScale3D (Variables|Default|GetPlane) "2.500000,2.500000,2.500000")
  (Transformation|SetWorldScale3D (Variables|Default|GetStaticMesh) "2.500000,2.500000,2.500000")
  (Transformation|SetWorldScale3D (Variables|Default|GetStaticMesh1) "2.500000,2.500000,2.500000")
  (Transformation|SetWorldLocation _staticmesh (- (Transformation|GetWorldLocation _staticmesh) "50.000000,0.000000,0.000000") false false)
  (Transformation|SetWorldLocation _staticmesh1 (+ (Transformation|GetWorldLocation _staticmesh1) "50.000000,0.000000,0.000000") false false)
  (Utilities|FlowControl|Delay 0.15)
  (Rendering|SetVisibility (Variables|Default|GetPlane) false false)
  (Rendering|SetVisibility (Variables|Default|GetStaticMesh) false false)
  (Rendering|SetVisibility (Variables|Default|GetStaticMesh1) false false))

(event Collision|EventActorBeginOverlap
  (params (OtherActor :type Actor%20Object%20Reference)))

(event EventTick
  (params (DeltaSeconds :type Float%20%28single-precision%29)))

(fn ConstructionScript)