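; Mushroom actor that continuously glides toward the location of a referenced target box.
; Each Tick calls the Avance event, which uses VInterpTo to ease the actor toward TargetBoxRef's current position, without sweep collision.
; BeginPlay stores the starting location in InitialVector, which these graphs never read.
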(event Custom|Avance
  (Transformation|SetActorLocation (Math|Interpolation|VInterpTo (Transformation|GetActorLocation) (Transformation|GetActorLocation (Variables|Default|GetTargetBoxRef)) (Utilities|Time|GetWorldDeltaSeconds) 2.0) false false))

(event EventBeginPlay
  (Variables|Default|SetInitialVector (Transformation|GetActorLocation)))

(event Collision|EventActorBeginOverlap
  (params (OtherActor :type Actor%20Object%20Reference)))

(event EventTick
  (params (DeltaSeconds :type Float%20%28single-precision%29))
  (CallFunction|Avance))

(fn ConstructionScript)