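; BP_BouncePadMovable is an actor, named as a movable bounce pad, that shuttles back and forth along the world X axis.
; BeginPlay calls the parent, then starts Right, whose timeline adds a fixed X offset on each update.
; On finish it calls Left, which reverses the offset and hands back to Right in an endless loop.
; The timelines act only as timers, so travel distance depends on frame rate.
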(event Custom|Right
  (Timeline|Timeline PlayFromStart
    (:Update
      (Transformation|SetActorLocation (+ (Transformation|GetActorLocation) "2.000000,0.000000,0.000000") false false))
    (:Finished
      (CallFunction|Left))))

(event Custom|Left
  (Timeline|Timeline_0 PlayFromStart
    (:Update
      (Transformation|SetActorLocation (- (Transformation|GetActorLocation) "2.000000,0.000000,0.000000") false false))
    (:Finished
      (CallFunction|Right))))

(event EventBeginPlay
  (|CallParentFunction)
  (CallFunction|Right))

(event Collision|EventActorBeginOverlap
  (params (OtherActor :type Actor%20Object%20Reference))
  (|CallParentFunction OtherActor) ; This node is disabled and will not be called.\nDrag off pins to build functionality.
)

(event EventTick
  (params (DeltaSeconds :type Float%20%28single-precision%29))
  (|CallParentFunction DeltaSeconds) ; This node is disabled and will not be called.\nDrag off pins to build functionality.
)

(fn ConstructionScript
  (|CallParentFunction))